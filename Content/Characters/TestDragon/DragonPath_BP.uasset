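; DragonPath_BP is a spline path actor, apparently for the test dragon, with editor orientation visualization and an end-window trigger.
; Its construction script optionally adds arrow components showing up and right vectors at each spline point, plus both vectors at segment midpoints.
; OpenEndWindowEvent checks that the end window reference is valid, waits a configurable delay, then activates that window.
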(event `OpenEndWindowEvent`
  (bind _refendwindow (`self.RefEndWindow`))
  (`/Engine/EditorBlueprintResources/StandardMacros.IsValid` _refendwindow
    (:`Is Valid`
      (`KismetSystemLibrary.Delay` (`self.TimeEnd`))
      (`/Game/SideScrollerBP/Blueprints/Window.ActiveWindowEvent` _refendwindow))))

(fn `UserConstructionScript`
  (bind _splinepath (`self.SplinePath`))
  (bind _splinepath_2 (`self.SplinePath`))
  (bind _returnvalue (`SplineComponent.GetNumberOfSplinePoints` (`self.SplinePath`)))
  (for _index (range (+ _returnvalue 1))
    (if (`self.ShowUpVector`)
      (bind _returnvalue_2 (`SplineComponent.GetLocationAtSplinePoint` _splinepath _index "Local"))
      (`AddComponent|NODE_AddArrowComponent-0` :`RelativeTransform` (`KismetMathLibrary.MakeTransform` _returnvalue_2 (`KismetMathLibrary.Conv_VectorToRotator` (`SplineComponent.GetUpVectorAtSplinePoint` _splinepath _index "Local")))))
    (if (`self.ShowRightVector`)
      (`AddComponent|NODE_AddArrowComponent-1` :`RelativeTransform` (`KismetMathLibrary.MakeTransform` _returnvalue_2 (`KismetMathLibrary.Conv_VectorToRotator` (`SplineComponent.GetRightVectorAtSplinePoint` _splinepath _index "Local")))))
    (if (`self.ShowVectorAlongPath`)
      (if (!= _index _returnvalue)
        (bind _returnvalue_3 (/ (+ (`SplineComponent.GetDistanceAlongSplineAtSplinePoint` _splinepath_2 (+ _index 1)) (`SplineComponent.GetDistanceAlongSplineAtSplinePoint` _splinepath_2 _index)) 2.0))
        (bind _returnvalue_4 (`SplineComponent.GetLocationAtDistanceAlongSpline` _splinepath_2 _returnvalue_3 "Local"))
        (`AddComponent|NODE_AddArrowComponent-2` :`RelativeTransform` (`KismetMathLibrary.MakeTransform` _returnvalue_4 (`KismetMathLibrary.Conv_VectorToRotator` (`SplineComponent.GetUpVectorAtDistanceAlongSpline` _splinepath_2 _returnvalue_3 "Local"))))
        (`AddComponent|NODE_AddArrowComponent-3` :`RelativeTransform` (`KismetMathLibrary.MakeTransform` _returnvalue_4 (`KismetMathLibrary.Conv_VectorToRotator` (`SplineComponent.GetRightVectorAtDistanceAlongSpline` _splinepath_2 _returnvalue_3 "Local"))))))))