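; Layered lamp-sky backdrop built from up to three planes, each with its own M_SkyLamp dynamic material.
; The construction script varies UV scale, emissive intensity and plane scale per layer for depth, destroying planes beyond Amount.
; A wave timeline drives horizontal speed at different rates per layer.
; Bound speed-boost and color-shift events play timelines that advance the vertical offset and blend the lamp tint to the new color.
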(event `self.ReceiveBeginPlay`
  (bind _speedx (`self.SpeedX`))
  (add `self.SpeedBoost` (delegate `SpeedShiftEvent`))
  (add `self.ColorShift` (delegate `ColorShiftEvent`))
  ;[1 1 1] WavyMovement
  (bind (_direction _wavefloat) (`Timeline|WaveAnimation`)
    (:`Update`
      (`MaterialInstanceDynamic.SetScalarParameterValue` (`self.Material1`) "Speed X" (* (* _wavefloat 1.0) _speedx))
      (`MaterialInstanceDynamic.SetScalarParameterValue` (`self.Material2`) "Speed X" (* (* _wavefloat 0.35) _speedx))
      (`MaterialInstanceDynamic.SetScalarParameterValue` (`self.Material3`) "Speed X" (* (* _wavefloat 0.3) _speedx)))))

(event `SpeedShiftEvent` :!signature `self.SpeedBoost`
  (params (NewSpeed :type "Float (double-precision)"))
  ;[1 1 1] Speed Shift
  (bind (_direction _offset_valur) (`Timeline|SpeedShiftAnimation` :!via `PlayFromStart`)
    (:`Update`
      (bind _output_get (set `self.OffsetY` (+ (`self.OffsetY`) _offset_valur)))
      (`MaterialInstanceDynamic.SetScalarParameterValue` (`self.Material1`) "Offset Y" _output_get)
      (`MaterialInstanceDynamic.SetScalarParameterValue` (`self.Material2`) "Offset Y" _output_get)
      (`MaterialInstanceDynamic.SetScalarParameterValue` (`self.Material3`) "Offset Y" _output_get))))

(event `ColorShiftEvent` :!signature `self.ColorShift`
  (params (NewColor :type "LinearColor Structure"))
  ;[1 1 1] Color Shift
  (bind (_direction _alpha) (`Timeline|ColorShiftAnimation` :!via `PlayFromStart`)
    (:`Update`
      (bind _returnvalue (`KismetMathLibrary.LinearColorLerp` (`self.LampsTint`) NewColor _alpha))
      (`MaterialInstanceDynamic.SetVectorParameterValue` (`self.Material1`) "LampTint" _returnvalue)
      (`MaterialInstanceDynamic.SetVectorParameterValue` (`self.Material2`) "LampTint" _returnvalue)
      (`MaterialInstanceDynamic.SetVectorParameterValue` (`self.Material3`) "LampTint" _returnvalue))
    (:`Finished`
      (set `self.LampsTint` NewColor))))

(fn `UserConstructionScript`
  (bind _material2 (`self.Material2`))
  (bind _uvscale (`self.UVScale`))
  (bind _material3 (`self.Material3`))
  (bind _lampstint (`self.LampsTint`))
  (bind _emissiveintensity (`self.EmissiveIntensity`))
  (bind _emissivediference (`self.EmissiveDiference`))
  (bind _returnvalue (+ (`self.UVScale`) (`self.UVScaleDiference`)))
  (bind _returnvalue_2 (+ (`self.UVScale`) (* (`self.UVScaleDiference`) 1.5)))
  ;[1 1 1] Create Materials and set UV scale
  (bind _returnvalue_3 (`KismetMaterialLibrary.CreateDynamicMaterialInstance` "/Game/Blueprints/LampSky/M_SkyLamp.M_SkyLamp" "None"))
  (bind _output_get (set `self.Material1` _returnvalue_3))
  (`PrimitiveComponent.SetMaterial` (`self.SkyPlane1`) 0 _output_get)
  (`MaterialInstanceDynamic.SetScalarParameterValue` (`self.Material1`) "U" _uvscale)
  (`MaterialInstanceDynamic.SetScalarParameterValue` _output_get "V" _uvscale)
  (`MaterialInstanceDynamic.SetScalarParameterValue` (`self.Material1`) "V" _uvscale)
  (bind _returnvalue_4 (`KismetMaterialLibrary.CreateDynamicMaterialInstance` "/Game/Blueprints/LampSky/M_SkyLamp.M_SkyLamp"))
  (bind _output_get_2 (set `self.Material2` _returnvalue_4))
  (`PrimitiveComponent.SetMaterial` (`self.SkyPlane2`) 0 _output_get_2)
  (`MaterialInstanceDynamic.SetScalarParameterValue` _material2 "U" _returnvalue)
  (`MaterialInstanceDynamic.SetScalarParameterValue` _material2 "V" _returnvalue)
  (bind _returnvalue_5 (`KismetMaterialLibrary.CreateDynamicMaterialInstance` "/Game/Blueprints/LampSky/M_SkyLamp.M_SkyLamp"))
  (bind _output_get_3 (set `self.Material3` _returnvalue_5))
  (`PrimitiveComponent.SetMaterial` (`self.SkyPlane3`) 0 _output_get_3)
  (`MaterialInstanceDynamic.SetScalarParameterValue` _material3 "U" _returnvalue_2)
  (`MaterialInstanceDynamic.SetScalarParameterValue` _material3 "V" _returnvalue_2)
  (`MaterialInstanceDynamic.SetScalarParameterValue` _material3 "Offset X" 0.2)
  ;[1 1 1] Set Speed
  (`MaterialInstanceDynamic.SetScalarParameterValue` (`self.Material1`) "Speed Multiplier" (`self.Speed`))
  (`MaterialInstanceDynamic.SetScalarParameterValue` (`self.Material2`) "Speed Multiplier" (`self.Speed`))
  (`MaterialInstanceDynamic.SetScalarParameterValue` (`self.Material3`) "Speed Multiplier" (`self.Speed`))
  ;[1 1 1] Emissive Intensity
  (`MaterialInstanceDynamic.SetScalarParameterValue` (`self.Material1`) "Emissive Intensity" _emissiveintensity)
  (`MaterialInstanceDynamic.SetScalarParameterValue` (`self.Material2`) "Emissive Intensity" (- _emissiveintensity _emissivediference))
  (`MaterialInstanceDynamic.SetScalarParameterValue` (`self.Material3`) "Emissive Intensity" (- _emissiveintensity (* _emissivediference 1.5)))
  ;[1 1 1] Setcolor
  (`MaterialInstanceDynamic.SetVectorParameterValue` (`self.Material1`) "LampTint" _lampstint)
  (`MaterialInstanceDynamic.SetVectorParameterValue` (`self.Material2`) "LampTint" _lampstint)
  (`MaterialInstanceDynamic.SetVectorParameterValue` (`self.Material3`) "LampTint" _lampstint)
  ;[1 1 1] Set Mesh
  (bind _output_get_4 (set `self.Planes` (`|MakeArray` (`self.SkyPlane1`) (`self.SkyPlane2`) (`self.SkyPlane3`))))
  (for (_array_element _array_index) _output_get_4
    (if (< _array_index (`self.Amount`))
      (bind _returnvalue_6 (* (+ (* _array_index (`self.ScaleDifference`)) 1.0) (`self.Scale`)))
      (`SceneComponent.SetRelativeScale3D` _array_element (`KismetMathLibrary.MakeVector` _returnvalue_6 _returnvalue_6 _returnvalue_6))
      (else
        (`ActorComponent.K2_DestroyComponent` _array_element)))))