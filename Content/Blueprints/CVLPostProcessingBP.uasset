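; Post-processing Blueprint that applies the player's saved colour options to the PostProcessBlur settings.
; On BeginPlay it binds to the UpdatePPValues dispatcher, then loads the PostProcessing save slot as OptionsSaveBP.
; The first three option values become uniform RGB saturation, contrast and gain, and each dispatcher call reloads and reapplies them.
; A separate EndGameSettings event also writes to those settings, with no values shown.
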(event `self.ReceiveBeginPlay`
  (add `self.UpdatePPValues` (delegate `UpdatePPValuesEvent`))
  (bind _returnvalue (`GameplayStatics.LoadGameFromSlot` "PostProcessing" :!label _label))
  (bind _asoptions_save_bp (cast `/Game/UI/MainMenu/OptionsSaveBP` _returnvalue))
  (bind _optionsvalues (`/Game/UI/MainMenu/OptionsSaveBP.OptionsValues` _asoptions_save_bp))
  (bind _output (`|GetArrayItem` _optionsvalues))
  (bind _output_2 (`|GetArrayItem` _optionsvalues 1))
  (bind _output_3 (`|GetArrayItem` _optionsvalues 2))
  (setmembers `PostProcessSettings` :`StructRef` (`PostProcessComponent.Settings` (`self.PostProcessBlur`)) :`ColorSaturation` (`KismetMathLibrary.MakeVector4` _output _output _output 1.0) :`ColorContrast` (`KismetMathLibrary.MakeVector4` _output_2 _output_2 _output_2 1.0) :`ColorGain` (`KismetMathLibrary.MakeVector4` _output_3 _output_3 _output_3 1.0)))

(event `UpdatePPValuesEvent`
  (goto _label))

(event `EndGameSettings`
  (setmembers `PostProcessSettings` :`StructRef` (`PostProcessComponent.Settings` (`self.PostProcessBlur`))))

(fn `UserConstructionScript`)