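; LampLight is a light actor whose point light flickers by continually drifting around its starting intensity.
; Each cycle picks a random target within RandomRange of that intensity and plays a timeline, at a slightly randomized Speed, to lerp toward it.
; On finish it stores the current intensity and, after a zero-length delay, calls the PlayTimeline dispatcher bound at BeginPlay to start the next cycle.
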(event `self.ReceiveBeginPlay`
  (bind _output_get (set `self.initialIntensity` (`LightComponentBase.Intensity` (`self.PointLightComponent`))))
  (set `self.currentIntensity` _output_get)
  (add `self.PlayTimeline` (delegate `PlayTimelineEvent`))
  (`self.PlayTimelineEvent`))

(event `PlayTimelineEvent`
  (bind _initialintensity (`self.initialIntensity`))
  (bind _randomrange (`self.randomRange`))
  (set `self.newIntensity` (`KismetMathLibrary.RandomFloatInRange` (- _initialintensity _randomrange) (+ _initialintensity _randomrange)))
  (`TimelineComponent.SetPlayRate` (`self.Alpha Timeline`) (* (`self.speed`) (`KismetMathLibrary.RandomFloatInRange` 0.8 1.2)))
  (bind (_direction _alpha) (`Timeline|Alpha Timeline` :!via `PlayFromStart`)
    (:`Update`
      (`LightComponent.SetIntensity` (`self.PointLightComponent`) (`KismetMathLibrary.Lerp` (`self.currentIntensity`) (`self.newIntensity`) _alpha)))
    (:`Finished`
      (set `self.currentIntensity` (`LightComponentBase.Intensity` (`self.PointLightComponent`)))
      (`KismetSystemLibrary.Delay` 0.0)
      (`self.PlayTimeline`))))

(fn `UserConstructionScript`)